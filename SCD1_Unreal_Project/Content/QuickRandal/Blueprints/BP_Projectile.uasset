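; BP_Projectile is a projectile actor that damages what it overlaps and then destroys itself.
; On overlap it ignores its Instigator and non-damageable actors, otherwise applying its Damage value credited to the instigator's controller.
; Any Hit event also destroys it, without applying damage.
; The construction script tints the Sphere red through the Color material parameter.
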(event EventBeginPlay)

(event Collision|EventActorBeginOverlap
  (params (OtherActor :type Actor%20Object%20Reference))
  (if (and (!= OtherActor (Variables|Actor|GetInstigator)) (Variables|/Script/Engine.Actor|GetbCanBeDamaged OtherActor))
    (Game|Damage|ApplyDamage OtherActor (Variables|Default|GetDamage) (Game|GetInstigatorController) self)
    (Actor|DestroyActor)))

(event EventTick
  (params (DeltaSeconds :type Float%20%28single-precision%29)))

(event Collision|EventHit
  (params (MyComp :type Primitive%20Component%20Object%20Reference) (Other :type Actor%20Object%20Reference) (OtherComp :type Primitive%20Component%20Object%20Reference) (bSelfMoved :type Boolean) (HitLocation :type Vector :default "0, 0, 0") (HitNormal :type Vector :default "0, 0, 0") (NormalImpulse :type Vector :default "0, 0, 0") (Hit :type Hit%20Result%20Structure%20%28by%20ref%29))
  (Actor|DestroyActor))

(fn ConstructionScript
  (Rendering|Material|SetVectorParameterValueonMaterials (Variables|Default|GetSphere) "Color" "1.000000, 0, 0"))