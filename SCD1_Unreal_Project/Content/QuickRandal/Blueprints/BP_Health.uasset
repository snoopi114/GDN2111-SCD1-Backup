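; BP_Health is a health component that tracks damage taken by its owning actor.
; On BeginPlay it fills current health to the maximum and binds to the owner's OnTakeAnyDamage.
; Damage is subtracted and clamped, then the OnHurt dispatcher fires while health remains, or OnDeath once it reaches zero.
; GetHealthRatio returns current health as a fraction of the maximum.
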(event Custom|TakeDamage
  (params (DamagedActor :type Actor%20Object%20Reference) (Damage :type Float%20%28single-precision%29) (DamageType :type Damage%20Type%20Object%20Reference) (InstigatedBy :type Controller%20Object%20Reference) (DamageCauser :type Actor%20Object%20Reference))
  (bind _output_get (Variables|Default|SetCurrentHealth (Math|Float|Clamp(Float) (- (Variables|Default|GetCurrentHealth) Damage) 0.0 (Variables|Default|GetMaxHealth))))
  (if (> _output_get 0.0)
    (Default|CallOnHurt)
    (else
      (Default|CallOnDeath))))

(event EventBeginPlay
  (Variables|Default|SetCurrentHealth (Variables|Default|GetMaxHealth))
  (EventDispatchers|AssignOnTakeAnyDamage (Components|GetOwner) (delegate Custom|TakeDamage)))

(event EventTick
  (params (DeltaSeconds :type Float%20%28single-precision%29)))

(fn GetHealthRatio
  (return (/ (Variables|Default|GetCurrentHealth) (Variables|Default|GetMaxHealth))))