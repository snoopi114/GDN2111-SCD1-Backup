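; BP_MaxHealPowerUp is a power-up that fully restores a character's health.
; Its Activate override sets the character's health component to max health, refreshes the health color, then runs the parent activation.
; The construction script tints the sphere green through a material parameter, and the event graph holds only disabled default events.
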(event EventBeginPlay
  (|CallParentFunction) ; This node is disabled and will not be called.\nDrag off pins to build functionality.
)

(event Collision|EventActorBeginOverlap
  (params (OtherActor :type Actor%20Object%20Reference))
  (|CallParentFunction OtherActor) ; This node is disabled and will not be called.\nDrag off pins to build functionality.
)

(event EventTick
  (params (DeltaSeconds :type Float%20%28single-precision%29))
  (|CallParentFunction DeltaSeconds) ; This node is disabled and will not be called.\nDrag off pins to build functionality.
)

(fn ConstructionScript
  (|CallParentFunction)
  (Rendering|Material|SetVectorParameterValueonMaterials (Variables|Default|GetSphere) "Color" "0.000000,1.000000,0.000000"))

(fn Activate
  (params (Character :type Side%20Scroller%20Character%20Object%20Reference))
  (bind _bp_charhealth (Variables|/Game/SideScrollerBP/Blueprints/SideScrollerCharacter.SideScrollerCharacter_C|GetBP_CharHealth Character))
  (Variables|/Game/QuickRandal/Blueprints/BP_Health.BP_Health_C|SetCurrentHealth _bp_charhealth (Variables|/Game/QuickRandal/Blueprints/BP_Health.BP_Health_C|GetMaxHealth _bp_charhealth))
  (Default|UpdateHealthColor Character)
  (|CallParentFunction 0))